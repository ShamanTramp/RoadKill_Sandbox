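; Baby_BP is an AI-moved baby that heads for the player character until it reaches it.
; It targets the player on BeginPlay, and a Delay on Tick throttles repeated SimpleMoveToActor calls, re-acquiring the player if the target is invalid.
; A mesh hit or overlap with the target stops movement and sets TargetReached, ending the chase.
; Disconnected nodes hold unused logic for chaining babies behind one another.
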(event `self.ReceiveBeginPlay`
  (bind _output_get (set `self.CurrentTarget` (`GameplayStatics.GetPlayerCharacter` 0)))
  (`NavigationSystem.SimpleMoveToActor` (`self.GetController`) _output_get))

(event `self.ReceiveTick`
  (params (DeltaSeconds :type "Float (single-precision)"))
  (`KismetSystemLibrary.Delay` 0.2)
  (if (not (`self.TargetReached`))
    (if (not (`KismetSystemLibrary.IsValid` (`self.CurrentTarget`)))
      (set `self.CurrentTarget` (`GameplayStatics.GetPlayerCharacter` 0)))
    (`NavigationSystem.SimpleMoveToActor` (`self.GetController`) (`self.CurrentTarget`))))

(event `self.Mesh.OnComponentHit`
  (params (HitComponent :type "PrimitiveComponent Object Reference") (OtherActor :type "Actor Object Reference") (OtherComp :type "PrimitiveComponent Object Reference") (NormalImpulse :type "Vector Structure") (Hit :type "HitResult Structure (by ref)"))
  (if (== OtherActor (`self.CurrentTarget`))
    (`Controller.StopMovement` (`self.GetController`) :!label _label)
    (set `self.TargetReached` true)))

(event `self.Mesh.OnComponentBeginOverlap`
  (params (OverlappedComponent :type "PrimitiveComponent Object Reference") (OtherActor :type "Actor Object Reference") (OtherComp :type "PrimitiveComponent Object Reference") (OtherBodyIndex :type Integer) (bFromSweep :type Boolean) (SweepResult :type "HitResult Structure (by ref)"))
  (if (== OtherActor (`self.CurrentTarget`))
    (goto _label)))

(fn `UserConstructionScript`)