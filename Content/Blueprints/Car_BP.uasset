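; Car hazard that kills turtles on contact with its wheels, with all four wheel overlaps feeding one shared handler.
; An exact TurtleCharacter class match spawns an impact particle and dead-turtle sprite at the car.
; Baby_BP hits spawn repeated particles and a sprite, then destroy the baby.
; Otherwise, a living player gets launched along the car's forward vector with brake sound and particles, marked dead, and shown Game Over UI.
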(event `self.ReceiveTick`
  (params (DeltaSeconds :type "Float (single-precision)")))

(event `self.ReceiveBeginPlay`)

(event `self.Wheel_F_R.OnComponentBeginOverlap`
  (params (OverlappedComponent :type "PrimitiveComponent Object Reference") (OtherActor :type "Actor Object Reference") (OtherComp :type "PrimitiveComponent Object Reference") (OtherBodyIndex :type Integer) (bFromSweep :type Boolean) (SweepResult :type "HitResult Structure (by ref)"))
  (bind _returnvalue (`GameplayStatics.GetPlayerController` 0))
  (bind _returnvalue_2 (`GameplayStatics.GetPlayerCharacter` 0))
  (bind _returnvalue_3 (`self.GetTransform`))
  (bind _returnvalue_4 (`self.K2_GetActorLocation` _returnvalue_2))
  (if (or (== (`GameplayStatics.GetObjectClass` OtherActor) "/Game/Blueprints/TurtleCharacter.TurtleCharacter_C") (== (`GameplayStatics.GetObjectClass` (stale `self.Wheel_F_L.OnComponentBeginOverlap` OtherActor)) "/Game/Blueprints/TurtleCharacter.TurtleCharacter_C") (== (`GameplayStatics.GetObjectClass` (stale `self.Wheel_B_L.OnComponentBeginOverlap` OtherActor)) "/Game/Blueprints/TurtleCharacter.TurtleCharacter_C") (== (`GameplayStatics.GetObjectClass` (stale `self.Wheel_B_R.OnComponentBeginOverlap` OtherActor)) "/Game/Blueprints/TurtleCharacter.TurtleCharacter_C")) :!label _label
    (`GameplayStatics.SpawnEmitterAtLocation` "/Game/Particles/Particles/Blood/P_body_bullet_impact.P_body_bullet_impact" (.location _returnvalue_3) (`KismetMathLibrary.RandomRotator` true) (0.5 0.5 0.5))
    (`|SpawnActorFromClass` "/Game/Blueprints/DeadTurtle_Sprite_BP.DeadTurtle_Sprite_BP_C" (`KismetMathLibrary.MakeTransform` (`KismetMathLibrary.MakeVector` (.x (.location _returnvalue_3)) (.y (.location _returnvalue_3)) (- (.z (.location _returnvalue_3)) 5.0)) (`KismetMathLibrary.MakeRotator` (+ (.roll (.rotation _returnvalue_3)) 90.0) (.pitch (.rotation _returnvalue_3)) (- (.yaw (.rotation _returnvalue_3)) 20.0)) (0.05 0.05 0.05)) "Undefined" "OverrideRootScale" null null)
    (elif (or (== (`GameplayStatics.GetObjectClass` OtherActor) "/Game/Blueprints/Baby_BP.Baby_BP_C") (== (`GameplayStatics.GetObjectClass` (stale `self.Wheel_F_L.OnComponentBeginOverlap` OtherActor)) "/Game/Blueprints/Baby_BP.Baby_BP_C") (== (`GameplayStatics.GetObjectClass` (stale `self.Wheel_B_L.OnComponentBeginOverlap` OtherActor)) "/Game/Blueprints/Baby_BP.Baby_BP_C") (== (`GameplayStatics.GetObjectClass` (stale `self.Wheel_B_R.OnComponentBeginOverlap` OtherActor)) "/Game/Blueprints/Baby_BP.Baby_BP_C"))
      (bind _outactors (`GameplayStatics.GetAllActorsOfClass` "/Game/Blueprints/Baby_BP.Baby_BP_C"))
      (for _array_element _outactors
        (if (or (== _array_element OtherActor) (== _array_element (stale `self.Wheel_F_L.OnComponentBeginOverlap` OtherActor)) (== _array_element (stale `self.Wheel_B_L.OnComponentBeginOverlap` OtherActor)) (== _array_element (stale `self.Wheel_B_R.OnComponentBeginOverlap` OtherActor)))
          (`PrimitiveComponent.SetSimulatePhysics` (`Character.Mesh` _array_element) true)
          (cast `/Game/Blueprints/TurtleCharacter` (`GameplayStatics.GetPlayerCharacter` 0))
          (`|ExecutionSequence`
            (:`then_0`
              (bind _returnvalue_5 (`self.GetTransform` _array_element))
              (`GameplayStatics.SpawnEmitterAtLocation` "/Game/Particles/Particles/Blood/P_body_bullet_impact.P_body_bullet_impact" (.location _returnvalue_5) (`KismetMathLibrary.RandomRotator` true) (0.5 0.5 0.5) :!label _label_2))
            (:`then_1`
              (goto _label_2))
            (:`then_2`
              (goto _label_2))
            (:`then_3`
              (goto _label_2))
            (:`then_4`
              (goto _label_2))
            (:`then_5`
              (`|SpawnActorFromClass` "/Game/Blueprints/DeadTurtle_Sprite_BP.DeadTurtle_Sprite_BP_C" (`self.SpriteTransform` _returnvalue_5) "Undefined" "OverrideRootScale" null null)
              (`self.K2_DestroyActor` _array_element)))))
      (else
        (bind _asturtle_character (cast `/Game/Blueprints/TurtleCharacter` _returnvalue_2))
        (if (`/Game/Blueprints/TurtleCharacter.PlayerIsDead` _asturtle_character)
          _
          (elif (or (== _asturtle_character OtherActor) (== _asturtle_character (stale `self.Wheel_F_L.OnComponentBeginOverlap` OtherActor)) (== _asturtle_character (stale `self.Wheel_B_L.OnComponentBeginOverlap` OtherActor)) (== _asturtle_character (stale `self.Wheel_B_R.OnComponentBeginOverlap` OtherActor)))
            (`PrimitiveComponent.SetSimulatePhysics` (`Character.Mesh` _asturtle_character) true)
            (`GameplayStatics.PlaySoundAtLocation` "/Game/Audio/CarCustom/CarBrake.CarBrake" _returnvalue_4 (struct) 0.3 (`KismetMathLibrary.RandomFloatInRange` 0.75 1.0) 0.3)
            (`|ExecutionSequence`
              (:`then_0`
                (`PrimitiveComponent.AddImpulse` (`Character.Mesh` _asturtle_character) (* (`SceneComponent.GetForwardVector` (`self.Mesh`)) 1000.0) "None" false)
                (set `/Game/Blueprints/TurtleCharacter.PlayerIsDead` true _asturtle_character)
                (`ActorComponent.Deactivate` (`Character.CharacterMovement` _asturtle_character))
                (bind _returnvalue_6 (`|CreateWidget` "/Game/Blueprints/UI/Menus/GameOver_UI.GameOver_UI_C"))
                (bind _output_get (set `self.GameOver_UI` _returnvalue_6))
                (set `PlayerController.bShowMouseCursor` true _returnvalue)
                (`WidgetBlueprintLibrary.SetInputMode_UIOnlyEx` _returnvalue _output_get)
                (`WidgetLayoutLibrary.RemoveAllWidgets` _output_get)
                (`UserWidget.AddToViewport` _output_get 0))
              (:`then_1`
                (`GameplayStatics.SpawnEmitterAtLocation` "/Game/Particles/Particles/Blood/P_body_bullet_impact.P_body_bullet_impact" _returnvalue_4 (`KismetMathLibrary.RandomRotator` true) :!label _label_3))
              (:`then_2`
                (goto _label_3))
              (:`then_3`
                (goto _label_3))
              (:`then_4`
                (goto _label_3))
              (:`then_5`
                (goto _label_3)))))))))

(event `self.Wheel_F_L.OnComponentBeginOverlap`
  (params (OverlappedComponent :type "PrimitiveComponent Object Reference") (OtherActor :type "Actor Object Reference") (OtherComp :type "PrimitiveComponent Object Reference") (OtherBodyIndex :type Integer) (bFromSweep :type Boolean) (SweepResult :type "HitResult Structure (by ref)"))
  (goto _label))

(event `self.Wheel_B_L.OnComponentBeginOverlap`
  (params (OverlappedComponent :type "PrimitiveComponent Object Reference") (OtherActor :type "Actor Object Reference") (OtherComp :type "PrimitiveComponent Object Reference") (OtherBodyIndex :type Integer) (bFromSweep :type Boolean) (SweepResult :type "HitResult Structure (by ref)"))
  (goto _label))

(event `self.Wheel_B_R.OnComponentBeginOverlap`
  (params (OverlappedComponent :type "PrimitiveComponent Object Reference") (OtherActor :type "Actor Object Reference") (OtherComp :type "PrimitiveComponent Object Reference") (OtherBodyIndex :type Integer) (bFromSweep :type Boolean) (SweepResult :type "HitResult Structure (by ref)"))
  (goto _label))

(fn `UserConstructionScript`)