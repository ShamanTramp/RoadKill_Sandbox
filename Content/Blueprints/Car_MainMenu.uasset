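; Main-menu car that kills chickens when one of its wheels runs into a ChickenCharacter.
; All four wheel overlap events share one handler that spawns a blood splash at the car's location and destroys every ChickenCharacter in the level, not just the one hit.
; Unconnected leftover logic for running over Baby_BP and the turtle player, including ragdoll and game-over UI, never runs.
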(event `self.ReceiveBeginPlay`)

(event `self.ReceiveTick`
  (params (DeltaSeconds :type "Float (single-precision)")))

(event `self.Wheel_F_R.OnComponentBeginOverlap`
  (params (OverlappedComponent :type "PrimitiveComponent Object Reference") (OtherActor :type "Actor Object Reference") (OtherComp :type "PrimitiveComponent Object Reference") (OtherBodyIndex :type Integer) (bFromSweep :type Boolean) (SweepResult :type "HitResult Structure (by ref)"))
  (if (or (== (`GameplayStatics.GetObjectClass` OtherActor) "/Game/Blueprints/ChickenCharacter.ChickenCharacter_C") (== (`GameplayStatics.GetObjectClass` (stale `self.Wheel_F_L.OnComponentBeginOverlap` OtherActor)) "/Game/Blueprints/ChickenCharacter.ChickenCharacter_C") (== (`GameplayStatics.GetObjectClass` (stale `self.Wheel_B_L.OnComponentBeginOverlap` OtherActor)) "/Game/Blueprints/ChickenCharacter.ChickenCharacter_C") (== (`GameplayStatics.GetObjectClass` (stale `self.Wheel_B_R.OnComponentBeginOverlap` OtherActor)) "/Game/Blueprints/ChickenCharacter.ChickenCharacter_C")) :!label _label
    (`GameplayStatics.SpawnEmitterAtLocation` "/Game/Particles/Particles/Blood/P_blood_huge_splash.P_blood_huge_splash" (.location (`self.GetTransform`)) (`KismetMathLibrary.RandomRotator` true) (0.5 0.5 0.5))
    (bind _outactors (`GameplayStatics.GetAllActorsOfClass` "/Game/Blueprints/ChickenCharacter.ChickenCharacter_C"))
    (for _array_element _outactors
      (`self.K2_DestroyActor` _array_element))))

(event `self.Wheel_F_L.OnComponentBeginOverlap`
  (params (OverlappedComponent :type "PrimitiveComponent Object Reference") (OtherActor :type "Actor Object Reference") (OtherComp :type "PrimitiveComponent Object Reference") (OtherBodyIndex :type Integer) (bFromSweep :type Boolean) (SweepResult :type "HitResult Structure (by ref)"))
  (goto _label))

(event `self.Wheel_B_L.OnComponentBeginOverlap`
  (params (OverlappedComponent :type "PrimitiveComponent Object Reference") (OtherActor :type "Actor Object Reference") (OtherComp :type "PrimitiveComponent Object Reference") (OtherBodyIndex :type Integer) (bFromSweep :type Boolean) (SweepResult :type "HitResult Structure (by ref)"))
  (goto _label))

(event `self.Wheel_B_R.OnComponentBeginOverlap`
  (params (OverlappedComponent :type "PrimitiveComponent Object Reference") (OtherActor :type "Actor Object Reference") (OtherComp :type "PrimitiveComponent Object Reference") (OtherBodyIndex :type Integer) (bFromSweep :type Boolean) (SweepResult :type "HitResult Structure (by ref)"))
  (goto _label))

(fn `UserConstructionScript`)